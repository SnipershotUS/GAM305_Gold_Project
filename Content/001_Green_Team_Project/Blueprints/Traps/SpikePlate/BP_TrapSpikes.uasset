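; BP_TrapSpikes is a spike plate trap that moves its spikes and damages the player.
; When the player character overlaps the Trigger, a Timeline plays and drives the Z of the Spikes' relative location.
; Overlapping SpikeBox applies fixed damage, targeted at the player controller rather than the character.
; An author note marks the trigger logic as not yet working.
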(event OnComponentBeginOverlap(SpikeBox)
  (params (OverlappedComponent :type Primitive%20Component%20Object%20Reference) (OtherActor :type Actor%20Object%20Reference) (OtherComp :type Primitive%20Component%20Object%20Reference) (OtherBodyIndex :type Integer) (bFromSweep :type Boolean) (SweepResult :type Hit%20Result%20Structure%20%28by%20ref%29))
  (if (== OtherActor (Game|GetPlayerCharacter 0))
    (Game|Damage|ApplyDamage (Game|GetPlayerController 0) 1e+01 0 0)))

(event OnComponentBeginOverlap(Trigger)
  (params (OverlappedComponent :type Primitive%20Component%20Object%20Reference) (OtherActor :type Actor%20Object%20Reference) (OtherComp :type Primitive%20Component%20Object%20Reference) (OtherBodyIndex :type Integer) (bFromSweep :type Boolean) (SweepResult :type Hit%20Result%20Structure%20%28by%20ref%29))
  ;[0.15 0.15 0.15 0.5] Wasn't working for some reason. Still need to fix.
  (if (== OtherActor (Game|GetPlayerCharacter 0))
    (bind _newtrack_0 (Timeline|Timeline Play)
      (:Update
        (Transformation|SetRelativeLocation (Variables|Default|GetSpikes) (Math|Vector|MakeVector 0.0 0.0 _newtrack_0) false false)))))

(event EventBeginPlay)

(fn ConstructionScript)