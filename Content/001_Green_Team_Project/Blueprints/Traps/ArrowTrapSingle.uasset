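; ArrowTrapSingle is a trap Blueprint that repeatedly shoots arrows once triggered.
; Triggered fires an arrow immediately, then starts a looping timer that keeps calling ShootArrow at a fixed interval.
; ShootArrow spawns an Arrow at the ShootyHole component's location, passing Damage and the IsV1 flag, then flips that flag so successive shots alternate between two arrow varieties.
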(event Custom|ShootArrow
  ;[0.15 0.15 0.15 0.5] Shoot arrows
  (Game|SpawnActorfromClass "/Game/001_Green_Team_Project/Blueprints/Traps/Projectiles/Arrow.Arrow_C" (Math|Transform|MakeTransform (Transformation|GetWorldLocation (Variables|Default|GetShootyHole)) "0, 0, 0" "1.000000,1.000000,1.000000") "Undefined" "MultiplyWithRoot" 0 (Variables|Default|GetIsV1) (Variables|Default|GetDamage) 0)
  ;;[0.15 0.15 0.15 0.5] Switch Arrow variety
  (Variables|Default|SetIsV1 (not (Variables|Default|GetIsV1))))

(event Custom|Triggered
  (CallFunction|ShootArrow)
  (Utilities|Time|SetTimerbyEvent (delegate Custom|ShootArrow) 2.0 true))

(fn ConstructionScript)