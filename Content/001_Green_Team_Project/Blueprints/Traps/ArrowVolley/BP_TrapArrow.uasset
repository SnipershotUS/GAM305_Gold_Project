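; BP_TrapArrow is an arrow volley trap that springs when its trigger volume is overlapped.
; Any overlap with the trigger plays a timeline that drives the relative Z location of two arrow components, ArrowV1 and ArrowV2, on separate tracks.
; When either set of arrow tips overlaps the player character, it applies a small fixed damage, targeted at the player controller rather than the character.
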(event OnComponentBeginOverlap(Trigger)
  (params (OverlappedComponent :type Primitive%20Component%20Object%20Reference) (OtherActor :type Actor%20Object%20Reference) (OtherComp :type Primitive%20Component%20Object%20Reference) (OtherBodyIndex :type Integer) (bFromSweep :type Boolean) (SweepResult :type Hit%20Result%20Structure%20%28by%20ref%29))
  (bind (_direction _av1 _av2) (Timeline|Timeline Play)
    (:Update
      (Transformation|SetRelativeLocation (Variables|Default|GetArrowV2) (Math|Vector|MakeVector 0.0 0.0 _av2) false false)
      (Transformation|SetRelativeLocation (Variables|Default|GetArrowV1) (Math|Vector|MakeVector 0.0 0.0 _av1) false false))))

(event OnComponentBeginOverlap(ArrowV2Tips)
  (params (OverlappedComponent :type Primitive%20Component%20Object%20Reference) (OtherActor :type Actor%20Object%20Reference) (OtherComp :type Primitive%20Component%20Object%20Reference) (OtherBodyIndex :type Integer) (bFromSweep :type Boolean) (SweepResult :type Hit%20Result%20Structure%20%28by%20ref%29))
  (if (== OtherActor (Game|GetPlayerCharacter 0))
    (Game|Damage|ApplyDamage (Game|GetPlayerController 0) 5.0 0 0)))

(event OnComponentBeginOverlap(ArrowV1Tips)
  (params (OverlappedComponent :type Primitive%20Component%20Object%20Reference) (OtherActor :type Actor%20Object%20Reference) (OtherComp :type Primitive%20Component%20Object%20Reference) (OtherBodyIndex :type Integer) (bFromSweep :type Boolean) (SweepResult :type Hit%20Result%20Structure%20%28by%20ref%29))
  (if (== OtherActor (Game|GetPlayerCharacter 0))
    (Game|Damage|ApplyDamage (Game|GetPlayerController 0) 5.0 0 0)))

(fn ConstructionScript)