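; Base character with health, respawn, sprint, interact and melee, ranged or boss attacks.
; Interact, defend (print only) and attack share a DSE toggle that cancels sprint and changes movement scale.
; Melee and interact use line traces, ranged spawns a projectile, and delay-based flags gate attacks, spells and minions.
; Damage at half health starts phase 2, enabling boss minion summons alongside AOE spells; zero health calls OnDeath and destroys the actor.
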(event Custom|Interact
  (params (IsInteracting :type Boolean))
  ;[0.15 0.15 0.15 0.5] Interact
  (Utilities|ToggleDSE IsInteracting
    (:DSE
      (Utilities|Interacted))))

(event Custom|Sprint
  (params (IsSprinting :type Boolean))
  ;[0.15 0.15 0.15 0.5] Sprint
  (if IsSprinting
    (if (not (Variables|Movement|GetIsDSE))
      (Variables|Movement|SetIsSprinting true)
      (else
        (Variables|Movement|SetIsSprinting false :!label _label)))
    (else
      (goto _label))))

(event Custom|Respawn
  (Transformation|SetActorLocation (Variables|Positions|GetRespawnPosition) false false)
  (Development|PrintString "Respawn - do other stuff here too"))

(event Custom|CalculateMS
  (bind _movementspeed (Variables|Movement|GetMovementSpeed))
  ;[0.15 0.15 0.15 0.5] Depricated
  ;;[0.15 0.15 0.15 0.5] Calculte Movement Scale
  (if (Variables|Movement|GetIsDSE)
    (Variables|Movement|SetMovementScale (* (Variables|Movement|GetMovementSpeed) (Variables|Movement|GetDSEMultiplier)))
    (elif (Variables|Movement|GetIsSprinting)
      (Variables|Movement|SetMovementScale (* _movementspeed (Variables|Movement|GetSprintMultiplier)))
      (else
        (Variables|Movement|SetMovementScale _movementspeed)))))

(event Custom|ShootProjectile
  (params (Rotation :type Rotator))
  ;[0.15 0.15 0.15 0.5] Shoot a projectile
  (Game|SpawnActorfromClass "/Game/001_Green_Team_Project/Blueprints/_WorkInProgress/MatthewSandberg/Prototypes/Projectiles/Boner.Boner_C" (Math|Transform|MakeTransform (Transformation|GetActorLocation) Rotation "1.000000,1.000000,1.000000") "Undefined" "MultiplyWithRoot" 0 (Variables|Health|GetCurrentDamage) 0))

(event Custom|Attack
  (params (IsAttacking :type Boolean) (AttackType :type AttackType%20Enum :default "NewEnumerator0"))
  ;[0.15 0.15 0.15 0.5] Attack
  (Utilities|ToggleDSE IsAttacking
    (:DSE
      (Utilities|Attacked AttackType))))

(event Custom|OnDeath
  ;[0.15 0.15 0.15 0.5] Header Function
)

(event Custom|Defend
  (params (IsDefending :type Boolean))
  ;[0.15 0.15 0.15 0.5] Defend
  (Utilities|ToggleDSE IsDefending
    (:DSE
      (Development|PrintString "I am DEFENDING"))))

(event Custom|Restart
  (Variables|Positions|SetRespawnPosition (Variables|Positions|GetOriginalPosition))
  (CallFunction|Respawn))

(event EventTakeDamage
  (params (Damage :type Float%20%28double-precision%29))
  ;[0.15 0.15 0.15 0.5] Depricated
  ;;[0.15 0.15 0.15 0.5] Take Damage from interface
  (Development|PrintString (Utilities|String|Append (Utilities|String|Append (Utilities|String|Append "Damage done to " (Utilities|GetObjectName self)) ": ") (Utilities|String|ToString(Float) Damage))))

(event Game|Damage|EventAnyDamage
  (params (Damage :type Float%20%28single-precision%29) (DamageType :type Damage%20Type%20Object%20Reference) (InstigatedBy :type Controller%20Object%20Reference) (DamageCauser :type Actor%20Object%20Reference))
  ;[0.15 0.15 0.15 0.5] Update character health when taking damage
  ;[0.15 0.15 0.15 0.5] Print Damage done
  (Development|PrintString (Utilities|String|Append (Utilities|String|Append (Utilities|String|Append "Damage done to " (Utilities|GetObjectName self)) ": ") (Utilities|String|ToString(Float) Damage)))
  (bind _output_get (Variables|Health|SetHealth (- (Variables|Health|GetHealth) Damage)))
  (if (<= _output_get (/ (Variables|Health|GetMaxHealth) 2.0))
    (Variables|Debug|SetPhase2Started true))
  (if (<= _output_get 0.0)
    (CallFunction|OnDeath)
    (Actor|DestroyActor)))

(fn ConstructionScript
  (bind _returnvalue (Transformation|GetActorLocation))
  (bind _charactermovement (Variables|Character|GetCharacterMovement))
  (Variables|Positions|SetRespawnPosition _returnvalue)
  (Variables|Positions|SetOriginalPosition _returnvalue)
  (Variables|Health|SetHealth (Variables|Health|GetMaxHealth))
  (Variables|Health|SetCurrentDamage (Variables|Health|GetBaseDamage))
  (bind _output_get (Variables|/Script/Engine.CharacterMovementComponent|SetMaxWalkSpeed _charactermovement (Variables|Movement|GetMaxSpeed)))
  (Variables|/Script/Engine.CharacterMovementComponent|SetMaxWalkSpeedCrouched _charactermovement (/ _output_get 2.0)))

(fn SpawnMinion
  (bind _randomlocation (Class|NavigationSystemV1|GetRandomLocationinNavigableRadius (Transformation|GetActorLocation) (Variables|Boss|GetMinionSpawnRadius) 0 0))
  (Game|SpawnActorfromClass "/Game/001_Green_Team_Project/Blueprints/Characters/Enemy/Created/Minion.Minion_C" (Math|Transform|MakeTransform _randomlocation "0, 0, 0" "1.000000,1.000000,1.000000") "Undefined" "MultiplyWithRoot" 0 0)
  (CallFunction|StartMinionTimer))

(fn SpawnSpell
  (Game|SpawnActorfromClass "/Game/001_Green_Team_Project/Blueprints/_WorkInProgress/MatthewSandberg/Prototypes/Projectiles/SpellAOE.SpellAOE_C" (Math|Transform|MakeTransform (Transformation|GetActorLocation (Variables|Main|GetTargetCharacter)) "0, 0, 0" "1.000000,1.000000,1.000000") "Undefined" "MultiplyWithRoot" 0 0)
  (CallFunction|StartSpellTimer))

(event Custom|StartSpellTimer
  ;[0.15 0.15 0.15 0.5] Spell timer
  (if (Variables|Boss|GetCanDoSpell)
    (Variables|Boss|SetCanDoSpell false)
    (Utilities|FlowControl|Delay (Variables|Boss|GetSpellDelayTime))
    (Variables|Boss|SetCanDoSpell true)))

(event Custom|StartMinionTimer
  ;[0.15 0.15 0.15 0.5] Minion timer
  (if (Variables|Boss|GetCanSummonMinion)
    (Variables|Boss|SetCanSummonMinion false)
    (Utilities|FlowControl|Delay (Variables|Boss|GetMinionDelayTime))
    (Variables|Boss|SetCanSummonMinion true)))

(event Custom|MeleeAttack
  (bind _attackdistance (Variables|Distances|GetAttackDistance))
  (bind (_start _end) (Utilities|GetVectoratDistance _attackdistance))
  ;[0.15 0.15 0.15 0.5] Melee Attack
  (Utilities|FlowControl|Delay (Variables|Timers|GetMeleeAttackDelayTime))
  (bind _outhit (Collision|LineTraceByChannel _start _end "TraceTypeQuery2" false 0 "ForDuration"))
  (Utilities|Casting|CastToBP_TopDownCharacter (.HitActor (Collision|BreakHitResult _outhit))
    (:then
      (Game|Damage|ApplyDamage (Game|GetPlayerController 0) (Variables|Health|GetCurrentDamage) 0 0)
      (Development|PrintString "Attacked a thing (melee)"))
    (:CastFailed
      (Development|PrintString "Did not hit anything (melee)"))))

(event Custom|RangedAttack
  ;[0.15 0.15 0.15 0.5] Ranged Attack
  (Utilities|FlowControl|Delay (Variables|Timers|GetRangedAttackDelayTime))
  (CallFunction|ShootProjectile (Transformation|GetActorRotation)))

(event Custom|StartAttackTimer
  ;[0.15 0.15 0.15 0.5] Attack Timer
  (if (Variables|Main|GetCanDoAttack)
    (Variables|Main|SetCanDoAttack false)
    (Variables|Main|SetIsAttacking true)
    (Utilities|FlowControl|Delay (Variables|Timers|GetAttackDelayTime))
    (Variables|Main|SetCanDoAttack true)
    (Variables|Main|SetIsAttacking false)))

(event Custom|BossAttack
  ;[0.15 0.15 0.15 0.5] Boss Attack
  (if (Variables|Debug|GetPhase2Started)
    (if (Variables|Boss|GetCanSummonMinion)
      (CallFunction|SpawnMinion)))
  (if (Variables|Boss|GetCanDoSpell)
    (CallFunction|SpawnSpell)))